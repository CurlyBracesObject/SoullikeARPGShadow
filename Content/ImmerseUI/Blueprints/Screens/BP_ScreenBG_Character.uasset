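; Screen background actor for the character menu, wrapping a character screen actor held in a child actor component.
; While the screen is open it takes player input, turning horizontal look input into rotation of the current target, scaled by a sensitivity value.
; Switching characters forwards the target to the child actor, and both switching and closing reset the child actor to its initial relative rotation.
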(event `self.ReceiveBeginPlay`
  (bind _asbp_character_screen_actor (cast `/Game/ImmerseUI/Blueprints/CharacterCustom/BP_CharacterScreenActor` (`ChildActorComponent.ChildActor` (`self.ChildActor`))))
  (set `self.Character` _asbp_character_screen_actor)
  (set `self.InitialRelativeRotation` (`SceneComponent.RelativeRotation` (`self.ChildActor`))))

(event `EnhancedInput|/Game/ImmerseUI/MenuInput/Actions/IA_LookMenu`
  (params (ActionValue :type "Vector2D Structure") (ElapsedSeconds :type "Float (double-precision)") (TriggeredSeconds :type "Float (double-precision)") (InputAction :type "InputAction Object Reference" :default "/Game/ImmerseUI/MenuInput/Actions/IA_LookMenu.IA_LookMenu"))
  (:`Triggered`
    (`/Game/ImmerseUI/Blueprints/CharacterCustom/BP_CharacterScreenActor.RotateCurrentTarget` (`self.Character`) (* (* ActionValue_X -1.0) (`self.RotateSensitivity`)))))

(event `self.OnOpen`
  (`self.EnableInput` (`GameplayStatics.GetPlayerController` 0)))

(event `self.OnClose`
  (`self.DisableInput` (`GameplayStatics.GetPlayerController` 0))
  (`self.OnExitSection`))

(event `OnExitSection`
  (`SceneComponent.K2_SetRelativeRotation` (`self.ChildActor`) (`self.InitialRelativeRotation`) false false))

(event `ChangeCharacter`
  (params (Target :type "/Game/ImmerseUI/Blueprints/Data/E_CharacterScreenTarget Enum" :default "NewEnumerator0"))
  (`/Game/ImmerseUI/Blueprints/CharacterCustom/BP_CharacterScreenActor.SwitchTarget` (`self.Character`) Target)
  (`self.OnExitSection`))

(fn `UserConstructionScript`
  (`parent.UserConstructionScript`))
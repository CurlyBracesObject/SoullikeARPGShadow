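; Background actor for UI screens that shifts its BG component as the cursor changes direction, when mouse movement is enabled.
; BeginPlay deactivates its CineCamera and binds MoveBackground to the CursorDirectionComponent's direction-change event.
; Each change restarts a rate-adjustable timeline that lerps BG toward an offset along that direction, passing Y and Z through horizontal and vertical clamp helpers.
; OnOpen and OnClose are empty events.
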(event `self.ReceiveBeginPlay`
  (`ActorComponent.SetActive` (`self.CineCamera`) false false)
  (add `/Game/ImmerseUI/Blueprints/BP_CursorDirection.OnDirectionChange` (`self.CursorDirectionComponent`) (delegate `MoveBackground`)))

(event `MoveBackground`
  (bind _maxhorizontalmovement (`self.MaxHorizontalMovement`))
  (bind _maxverticalmovement (`self.MaxVerticalMovement`))
  (bind _relativelocation (`SceneComponent.RelativeLocation` (`self.BG`)))
  (if (`self.UseMouseMovement`)
    (`TimelineComponent.SetPlayRate` (`self.TL_Move`) (`self.MovementRate`))
    (`/Game/ImmerseUI/Blueprints/BP_CursorDirection.DetectionSettings` (`self.CursorDirectionComponent`) (`self.DetectionSensitivity`))
    (`TimelineComponent.Stop` (`self.TL_Move`))
    (bind _cursor_direction (`/Game/ImmerseUI/Blueprints/BP_CursorDirection.GetDirection` (`self.CursorDirectionComponent`)))
    (set `self.TargetLocation` (+ (`SceneComponent.RelativeLocation` (`self.BG`)) (* _cursor_direction (`KismetMathLibrary.FMax` (`self.MaxHorizontalMovement`) (`self.MaxVerticalMovement`)))))
    (bind (_direction _t1) (`Timeline|TL_Move` :!via `PlayFromStart`)
      (:`Update`
        (bind (_returnvalue_x _returnvalue_y _returnvalue_z) (`KismetMathLibrary.BreakVector` (`KismetMathLibrary.VLerp` _relativelocation (`self.TargetLocation`) _t1)))
        (`SceneComponent.K2_SetRelativeLocation` (`self.BG`) (`KismetMathLibrary.MakeVector` (.x _relativelocation) (`KismetMathLibrary.FClamp` _returnvalue_y (* _maxhorizontalmovement -1.0) _maxhorizontalmovement) (`KismetMathLibrary.FClamp` _returnvalue_z (* _maxverticalmovement -1.0) _maxverticalmovement)) false false)))))

(event `OnOpen`)

(event `OnClose`)

(fn `UserConstructionScript`)
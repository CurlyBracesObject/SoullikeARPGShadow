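; Base GAS character that handles melee combos, directional dodges, target lock-on and dissolvable shadow afterimages.
; Loads combo, dodge and hit DataTables, then selects abilities from input and state gameplay tags, including movement-mode tags.
; Lock-on ranks nearby visible characters by yaw from the camera, steers control rotation and eases pitch back on release.
; Shadow copies skip ability setup; ASC callbacks relay added tags and destroy the actor when GA_Dead ends.
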(event Custom|Disolve%20Shadow
  ;[0.05098 0.05098 0.05098] 控制消散的方法
  ;;[0.05098 0.05098 0.05098] 消散前将材质切换为可以溶解的材质
  (Rendering|Material|SetMaterial (Variables|Character|GetMesh) 0 "/Game/Material_Niagara/M_PlanetRingDissolvable.M_PlanetRingDissolvable")
  (for _array_element (Components|GetChildrenComponents (Variables|Character|GetMesh) false)
    (bind _as基元组件 (Utilities|Casting|CastToPrimitiveComponent _array_element))
    (Rendering|Material|SetMaterial _as基元组件 0 "/Game/Material_Niagara/M_PlanetRingDissolvable.M_PlanetRingDissolvable")
    (bind _newtrack_0 (Timeline|Timeline_1 ReverseFromEnd)
      (:Update
        (Rendering|Material|SetScalarParameterValue "/Game/Material_Niagara/MPC_DissolveEdge.MPC_DissolveEdge" "Mask" _newtrack_0 :!class /Script/Engine.KismetMaterialLibrary)))))

(event Custom|Open%20Tag%20Cache
  (params (Listening%20Tag :type Gameplay%20Tag%20Structure))
  (Variables|Default|SetCacheTag "")
  (EventDispatchers|BindEventtoOnTagAdded (delegate Custom|Handle%20Added%20Tag)))

(event Custom|Handle%20Added%20Tag
  (params (Added%20Tag :type Gameplay%20Tag%20Structure))
  (if (GameplayTags|MatchesTag Added%20Tag (stale Custom|Open%20Tag%20Cache Listening%20Tag))
    (Variables|Default|SetCacheTag Added%20Tag)))

(event Custom|Reset%20Speed%20Smoothly
  ;[0.05098 0.05098 0.05098] 缓慢重设奔跑回复的速度
  (Variables|Default|SetLast%20Max%20Walk%20Speed (Variables|/Script/Engine.CharacterMovementComponent|GetMaxWalkSpeed (Variables|Character|GetCharacterMovement)))
  (bind _newtrack_0 (Timeline|Speed PlayFromStart)
    (:Update
      (Variables|/Script/Engine.CharacterMovementComponent|SetMaxWalkSpeed (Variables|Character|GetCharacterMovement) (Math|Float|Lerp (Variables|Default|GetLast%20Max%20Walk%20Speed) 5e+02 _newtrack_0)))))

(event Custom|Reactivate%20During%20Changing
  ;[0.05098 0.05098 0.05098] 缓慢重设奔跑回复的速度
  (bind _newtrack_0 (Timeline|Speed Stop)
    (:Update
      (Variables|/Script/Engine.CharacterMovementComponent|SetMaxWalkSpeed (Variables|Character|GetCharacterMovement) (Math|Float|Lerp (Variables|Default|GetLast%20Max%20Walk%20Speed) 5e+02 _newtrack_0)))))

(event EventOnMovementModeChanged
  (params (PrevMovementMode :type EMovementMode%20Enum :default "MOVE_None") (NewMovementMode :type EMovementMode%20Enum :default "MOVE_None") (PrevCustomMode :type Byte :default 0) (NewCustomMode :type Byte :default 0))
  ;[0.05098 0.05098 0.05098] 用于通知其他蓝图（如动画蓝图，移动状态改变）
  (Default|CallOnMovementModeChanged NewMovementMode)
  (switch Utilities|FlowControl|Switch|SwitchonEMovementMode NewMovementMode
    (:MOVE_Walking
      (GameplayTag|SwitchMovementTag "(TagName=\"Movement.Walk\")"))
    (:MOVE_NavWalking
      (GameplayTag|SwitchMovementTag "(TagName=\"Movement.NavWalk\")"))
    (:MOVE_Falling
      (GameplayTag|SwitchMovementTag "(TagName=\"Movement.Fly\")"))
    (:MOVE_Swimming
      (GameplayTag|SwitchMovementTag "(TagName=\"Movement.Swim\")"))
    (:MOVE_Flying
      (GameplayTag|SwitchMovementTag "(TagName=\"Movement.Fly\")"))
    (:MOVE_Custom
      (GameplayTag|SwitchMovementTag "(TagName=\"Movement.Custom\")"))))

(event EventBeginPlay
  (Utilities|FlowControl|Sequence
    (:then_1
      (if (not (Variables|Default|GetbIsShadow))
        (GameplayAbility|InitAbilities)
        (CallFunction|BindASCRelatedEvent)))))

(event EventTick
  (params (DeltaSeconds :type Float%20%28single-precision%29))
  (Utilities|FlowControl|Sequence
    (:then_0
      (DebugTools|PrintInfo (Variables|DebugVar|GetPrint%20INFO%20to%20Screen)))
    (:then_1
      (Development|PrintString (Utilities|GetDisplayName (Variables|CameraSystem|GetCurrentTarget)) true true "(R=1.000000,G=0.000000,B=0.111378,A=1.000000)" 0.02 "Target"))))

(event Input|KeyboardEvents|DebugKey1
  (params (Key :type Key%20Structure) (ActionValue :type Input%20Action%20Value%20Structure))
  (:Pressed
    (if (Variables|CameraSystem|GetIs%20Targeting)
      (CameraSystem|CameraTargetSwitch))))

(event Custom|Try%20Lock%20On%20Target
  ;[0.05098 0.05098 0.05098] 尝试锁敌
  (if (Variables|CameraSystem|GetIs%20Targeting)
    (CallFunction|LockOff)
    (else
      (bind _returnvalue (CameraSystem|GetAllSWGASActor))
      (if _returnvalue
        (bind _keys (Utilities|Map|Keys (Variables|CameraSystem|GetActors)))
        (bind _outhit (Collision|SphereTraceForObjects (Transformation|GetActorLocation) (Transformation|GetActorLocation (Utilities|Array|Get(acopy) _keys (.IndexOfMinValue (Math|Float|MinOfFloatArray (Variables|CameraSystem|GetCurrent%20Roatation))))) 25.0 (Utilities|Array|MakeArray "ObjectTypeQuery3") false (Utilities|Array|MakeArray self (Utilities|Array|Get(acopy) _keys (.IndexOfMinValue (Math|Float|MinOfFloatArray (Variables|CameraSystem|GetCurrent%20Roatation))))) "None"))
        (Utilities|Casting|CastToBP_SWGASCharacter (.HitActor (Collision|BreakHitResult _outhit))
          (:then
            (CallFunction|Lockon))
          (:CastFailed
            (CallFunction|Lockon (Utilities|Array|Get(acopy) _keys (.IndexOfMinValue (Math|Float|MinOfFloatArray (Variables|CameraSystem|GetCurrent%20Roatation)))))))))))

(event Custom|Lock%20On
  (params (Target :type BP%20SWGAS%20Character%20Object%20Reference))
  ;[0.05098 0.05098 0.05098] 开始锁定
  (Ability|GameplayEffect|AddLooseGameplayTags self (GameplayTags|MakeLiteralGameplayTagContainer "(GameplayTags=((TagName=\"State.Targeting\")))"))
  (Variables|CameraSystem|SetIs%20Targeting true)
  (bind _output_get (Variables|CameraSystem|SetCurrentTarget Target))
  (Default|CallOnTargetLockon _output_get)
  (Default|BeTargeted _output_get)
  (CameraSystem|SetCameraRotationMode false true false)
  ;[0.05098 0.05098 0.05098] 更新相机方法
  (Utilities|FlowControl|Gate true) ; enters at Open
)

(event Custom|Lock%20Off
  ;[0.05098 0.05098 0.05098] 结束锁定
  (Ability|GameplayEffect|RemoveLooseGameplayTags self (GameplayTags|MakeLiteralGameplayTagContainer "(GameplayTags=((TagName=\"State.Targeting\")))"))
  (Variables|CameraSystem|SetIs%20Targeting false)
  (bind _currenttarget (Variables|CameraSystem|GetCurrentTarget)
    (:then
      (Default|CallOnTargetLockon)
      (Default|RemoveTarget _currenttarget)
      (Variables|CameraSystem|SetCurrentTarget 0)
      (CameraSystem|SetCameraRotationMode false false true)
      (Utilities|FlowControl|Sequence
        (:then_0
          ;[0.05098 0.05098 0.05098] 更新相机方法
          (Utilities|FlowControl|Gate true) ; enters at Close
        )
        (:then_1
          (bind _rotation (Timeline|Timeline_0 PlayFromStart)
            (:Update
              (CallFunction|ResetCamera _rotation))))))
    (:else)))

(event Custom|Update%20Character%20Rotation
  (params (Delta%20Time :type Float%20%28double-precision%29) (InterpSpeed :type Float%20%28single-precision%29))
  (bind _returnvalue (Transformation|GetActorRotation))
  (bind (_roll _pitch) (Math|Rotator|BreakRotator _returnvalue))
  ;[0.05098 0.05098 0.05098] ANS驱动，调整角色在montage中的朝向
  (bind _currenttarget (Variables|CameraSystem|GetCurrentTarget)
    (:then
      (Transformation|SetActorRotation (Math|Interpolation|RInterpTo _returnvalue (Math|Rotator|MakeRotator _roll _pitch (.yaw (Math|Rotator|FindLookatRotation (Transformation|GetActorLocation) (Transformation|GetActorLocation _currenttarget)))) Delta%20Time InterpSpeed)))
    (:else)))

(event Custom|Set%20Camera%20Roatation
  (bind _returnvalue (Pawn|GetControlRotation :!class /Script/Engine.Pawn))
  (bind _camera (Variables|Default|GetCamera))
  (bind _currenttarget (Variables|CameraSystem|GetCurrentTarget))
  (bind _returnvalue_2 (Transformation|GetActorLocation _currenttarget))
  (bind _returnvalue_3 (Transformation|GetWorldLocation _camera))
  (bind _returnvalue_4 (Math|Rotator|FindLookatRotation _returnvalue_3 _returnvalue_2))
  ;[0.05098 0.05098 0.05098] 设置相机旋转
  (Pawn|SetControlRotation (Pawn|GetController) (Math|Interpolation|RInterpTo _returnvalue (Math|Rotator|MakeRotator (.Roll (Math|Rotator|BreakRotator _returnvalue)) (.pitch _returnvalue_4) (.yaw _returnvalue_4)) (Utilities|Time|GetWorldDeltaSeconds) (Variables|CameraSystem|GetInterp%20Speed))))

(event Custom|Stop%20Camera%20Reset
  ;[0.05098 0.05098 0.05098] 结束锁定
  (bind _rotation (Timeline|Timeline_0 Stop)
    (:Update
      (CallFunction|ResetCamera _rotation))))

(event Custom|Reset%20Camera
  (params (Alpha :type Float%20%28double-precision%29))
  (bind _returnvalue (Game|GetPlayerController 0))
  (bind _returnvalue_2 (Pawn|GetControlRotation _returnvalue :!class /Script/Engine.Controller))
  (bind (_roll _pitch _yaw) (Math|Rotator|BreakRotator _returnvalue_2))
  ;[0.05098 0.05098 0.05098] Reset Camera
  ;;[1 1 1] 如果有可以打断Camera 的条件放这里
  (if true
    (Pawn|SetControlRotation (Game|GetPlayerController 0) (Math|Rotator|Lerp(Rotator) _returnvalue_2 (Math|Rotator|MakeRotator _roll 0.0 _yaw) Alpha true))
    (else
      (CallFunction|StopCameraReset))))

(fn ConstructionScript)

(fn PrintInfo
  (params (bShouldPrint? :type Boolean))
  (bind _bpc_switchweaponasc (Variables|Default|GetBPC_SwitchWeaponASC))
  (if bShouldPrint?
    (Utilities|FlowControl|Sequence
      (:then_0
        (Utilities|Array|Clear (LocalVariables|GetPrint%20Message)))
      (:then_1
        ;[0.05098 0.05098 0.05098] 角色名字
        (Utilities|Array|Add (LocalVariables|GetPrint%20Message) (Utilities|GetDisplayName self)))
      (:then_2
        ;[0.05 0.05 0.05] 输出角色所有的Tag
        (LocalVariables|SetTemp%20Record " Tag: ")
        (for _array_element (.gameplaytags (GameplayTags|GetOwnedGameplayTags _bpc_switchweaponasc :!class /Script/GameplayTags.GameplayTagAssetInterface))
          (LocalVariables|SetTemp%20Record (Utilities|String|Append (LocalVariables|GetTemp%20Record) "&" (Utilities|String|ToString(Name) (GameplayTags|GetTagName _array_element)))))
        (Utilities|Array|Add (LocalVariables|GetPrint%20Message) (LocalVariables|GetTemp%20Record)))
      (:then_3
        ;[0.05098 0.05098 0.05098] 输出角色的所有Attribute
        (LocalVariables|SetTemp%20Record "")
        (for _array_element_2 (Class|AbilitySystemComponent|GetAllAttributes (Variables|Default|GetBPC_SwitchWeaponASC))
          (LocalVariables|SetTemp%20Record (Utilities|String|Append (LocalVariables|GetTemp%20Record) (Utilities|Struct|BreakGameplayAttribute _array_element_2) ":" (Utilities|String|ToString(Float) (.ReturnValue (Ability|Attribute|GetFloatAttributefromAbilitySystemComponent _bpc_switchweaponasc _array_element_2))) "&")))
        (Utilities|Array|Add (LocalVariables|GetPrint%20Message) (LocalVariables|GetTemp%20Record)))
      (:then_4
        ;[0.05098 0.05098 0.05098] 输出所有信息
        (for _array_element_3 (LocalVariables|GetPrint%20Message)
          (Development|PrintString _array_element_3 true true "(R=0.039546,G=0.651406,B=0.000000,A=1.000000)" (Utilities|Time|GetWorldDeltaSeconds)))))))

(fn OnTagChanged
  (params (Tag :type Gameplay%20Tag%20Structure%20%28by%20ref%29) (TagExists :type Boolean))
  ;[1 1 1] Tag Changed的回调函数，主要是用来做第二层的触发GA判定
  (if TagExists
    (Default|CallOnTagAdded Tag)))

(fn OnAbilityEnded
  (params (AbilityReference :type Gameplay%20Ability%20Object%20Reference) (wasCancelled :type Boolean))
  (if (== (Utilities|GetClass AbilityReference) "/Game/_GAS/GameplayAbilities/GA_Dead.GA_Dead_C")
    (Actor|DestroyActor)))

(fn OnGameplayAttributeChanged
  (params (Attribute :type Gameplay%20Attribute%20Structure) (Value :type Float%20%28single-precision%29)))

(fn SwitchMovementTag
  (params (New%20Movement%20Mode%20Tag :type Gameplay%20Tag%20Structure))
  (bind _self self)
  ;[1 1 1] 切换用于标识移动状态的Tag
  (Ability|GameplayEffect|RemoveLooseGameplayTags _self (GameplayTags|MakeLiteralGameplayTagContainer "(GameplayTags=((TagName=\"Movement.Custom\"),(TagName=\"Movement.Fall\"),(TagName=\"Movement.Fly\"),(TagName=\"Movement.NavWalk\"),(TagName=\"Movement.Walk\"),(TagName=\"Movement.Swim\")))"))
  (Ability|GameplayEffect|AddLooseGameplayTags _self (GameplayTags|MakeGameplayTagContainerfromTag New%20Movement%20Mode%20Tag)))

(fn TryFindExcuteComboAbility
  (params (InputAction%20Tag :type Gameplay%20Tag%20Structure))
  (bind _charactermovement (Variables|Character|GetCharacterMovement))
  (|SwitchGameplayTag InputAction%20Tag
    (:InputAction.Melee
      (for _array_element (Variables|Combat|GetCombo%20Data)
        (if (== (.TriggerInputActionTag (Utilities|Struct|BreakS_SingleAbilityInfo _array_element)) InputAction%20Tag)
          (LocalVariables|SetCombo%20Tag (.ComboTag (Utilities|Struct|BreakS_SingleAbilityInfo _array_element)))
          (if (and (or (== (LocalVariables|GetCombo%20Tag) "(TagName=\"Combo.Ground1\")") (GameplayTags|HasMatchingGameplayTag (Variables|Default|GetBPC_SwitchWeaponASC) (LocalVariables|GetCombo%20Tag))) (or (and (== (LocalVariables|GetCombo%20Tag) "(TagName=\"Combo.Ground1\")") (not (GameplayTags|HasMatchingGameplayTag (Variables|Default|GetBPC_SwitchWeaponASC) "(TagName=\"State.Attacking\")"))) (and (!= (LocalVariables|GetCombo%20Tag) "(TagName=\"Combo.Ground1\")") (GameplayTags|HasMatchingGameplayTag (Variables|Default|GetBPC_SwitchWeaponASC) "(TagName=\"State.Attacking\")"))))
            (return _array_element true))))
      (return "" false))
    (:InputAction.Dodge
      (Utilities|FlowControl|Sequence
        (:then_0
          (LocalVariables|SetbCanDodge (and (not (Class|NavMovementComponent|IsFlying _charactermovement)) (not (AI|Components|NavMovement|IsFalling _charactermovement))))
          (LocalVariables|SetbHasDodgeDir (GameplayTags|HasMatchingGameplayTag (Variables|Default|GetBPC_SwitchWeaponASC) "(TagName=\"InputAction.DodgeDir\")"))
          (LocalVariables|SetbIsTargeting (GameplayTags|HasMatchingGameplayTag (Variables|Default|GetBPC_SwitchWeaponASC) "(TagName=\"State.Targeting\")")))
        (:then_1
          (if (and (LocalVariables|GetbCanDodge) (LocalVariables|GetbIsTargeting))
            (if (LocalVariables|GetbHasDodgeDir)
              (for _array_element_2 (Variables|Dodge|GetDodge%20Data)
                (if (GameplayTags|HasMatchingGameplayTag (Variables|Default|GetBPC_SwitchWeaponASC) (.DodgeDirecitonTag (Utilities|Struct|BreakS_SingleAbilityInfo _array_element_2)))
                  (return _array_element_2 true)))
              (return "" false)
              (else
                ;[1 1 1] 锁定+无朝向
                (if true
                  (return (Variables|Dodge|GetBackward%20Dodge%20Data) true))))
            (elif (and (LocalVariables|GetbCanDodge) (not (LocalVariables|GetbIsTargeting)))
              (if (LocalVariables|GetbHasDodgeDir)
                (return (Variables|Dodge|GetForward%20Dodge%20Data) true)
                (elif true
                  (return (Variables|Dodge|GetBackward%20Dodge%20Data) true))))))))))

(fn ResetCombo
  (params (TagContainer :type Gameplay%20Tag%20Container%20Structure%20%28by%20ref%29))
  ;[0.05098 0.05098 0.05098] 删除原有的所有Combo Tag
  (Utilities|FlowControl|Sequence
    (:then_0
      (if (GameplayTags|HasAnyTags (GameplayTags|GetOwnedGameplayTags (Variables|Default|GetBPC_SwitchWeaponASC) :!class /Script/GameplayTags.GameplayTagAssetInterface) (GameplayTags|MakeLiteralGameplayTagContainer "(GameplayTags=((TagName=\"Combo\")))"))
        (Ability|GameplayEffect|RemoveLooseGameplayTags self (GameplayTags|MakeLiteralGameplayTagContainer "(GameplayTags=((TagName=\"Combo.Ground1\"),(TagName=\"Combo.Ground2\"),(TagName=\"Combo.Ground3\"),(TagName=\"Combo.Ground4\")))"))))
    (:then_1
      ;[0.05098 0.05098 0.05098] 添加新标签
      (Ability|GameplayEffect|AddLooseGameplayTags self TagContainer))))

(fn InitAbilities
  (Utilities|FlowControl|Sequence
    (:then_0
      ;[0.05098 0.05098 0.05098] 读取技能表格
      (bind _combo_data_table (Variables|Combat|GetCombo%20Data%20Table)
        (:then
          (bind _outrownames (DataTable|GetDataTableRowNames _combo_data_table))
          (for _array_element _outrownames
            (bind _returnvalue (Utilities|GetDataTableRow _combo_data_table _array_element)
              (:then
                (Utilities|Array|Add (Variables|Combat|GetCombo%20Data) _returnvalue)))))
        (:else)))
    (:then_1
      ;[0.05098 0.05098 0.05098] 读取翻滚表格
      (bind _dodge_data_table (Variables|Dodge|GetDodge%20Data%20Table)
        (:then
          (bind _outrownames_2 (DataTable|GetDataTableRowNames _dodge_data_table))
          (for _array_element_2 _outrownames_2
            (bind _returnvalue_2 (Utilities|GetDataTableRow _dodge_data_table _array_element_2)
              (:then
                (Utilities|Array|Add (Variables|Dodge|GetDodge%20Data) _returnvalue_2)
                (|SwitchGameplayTag (.DodgeDirecitonTag (Utilities|Struct|BreakS_SingleAbilityInfo _returnvalue_2))
                  (:InputAction.DodgeDir.F
                    (Variables|Dodge|SetForward%20Dodge%20Data _returnvalue_2))
                  (:InputAction.DodgeDir.B
                    (Variables|Dodge|SetBackward%20Dodge%20Data _returnvalue_2)))))))
        (:else)))
    (:then_2
      ;[0.05098 0.05098 0.05098] 读取受击表格
      (bind _hit_data_table (Variables|Combat|GetHit%20Data%20Table)
        (:then
          (bind _outrownames_3 (DataTable|GetDataTableRowNames _hit_data_table))
          (for _array_element_3 _outrownames_3
            (bind _returnvalue_3 (Utilities|GetDataTableRow _hit_data_table _array_element_3)
              (:then
                (Utilities|Array|Add (Variables|Combat|GetHit%20Data) _returnvalue_3)))))
        (:else)))
    (:then_3
      (return))))

(fn BindASCRelatedEvent
  (bind _bpc_switchweaponasc (Variables|Default|GetBPC_SwitchWeaponASC))
  (EventDispatchers|BindEventtoOnTagUpdatedDelegate _bpc_switchweaponasc (EventDispatchers|CreateEvent :!event OnTagChanged))
  (EventDispatchers|BindEventtoOnAbilityEndedBlueprintCallable _bpc_switchweaponasc (EventDispatchers|CreateEvent :!event OnAbilityEnded))
  (EventDispatchers|BindEventtoOnGameplayAttributeChanged _bpc_switchweaponasc (EventDispatchers|CreateEvent :!event OnGameplayAttributeChanged)))

(fn InitShadowSetting
  (bind _self self)
  (bind _returnvalue (AI|GetAIController _self))
  (if (Variables|Default|GetbIsShadow)
    (Utilities|FlowControl|Sequence
      (:then_0
        ;[0.05098 0.05098 0.05098] 初始化残影基本配置
        (Collision|SetCollisionEnabled (Variables|Default|GetCapsuleComponent) "NoCollision")
        (Pawn|Components|CharacterMovement|SetMovementMode (Variables|Character|GetCharacterMovement) "MOVE_Flying" 0)
        (Utilities|FlowControl|Sequence
          (:then_0
            (Utilities|IsValid _returnvalue
              (:Is%20Valid
                (Pawn|UnPossess _returnvalue))))))
      (:then_1
        ;[0.05098 0.05098 0.05098] 配置残影材质
        (Rendering|Material|SetMaterial (Variables|Character|GetMesh) 0 "/Game/Material_Niagara/M_PlanetRing.M_PlanetRing")
        (for _array_element (Components|GetChildrenComponents (Variables|Character|GetMesh) false)
          (bind _as基元组件 (Utilities|Casting|CastToPrimitiveComponent _array_element))
          (Rendering|Material|SetMaterial _as基元组件 0 "/Game/Material_Niagara/M_PlanetRing.M_PlanetRing")))
      (:then_2
        ;[0.05098 0.05098 0.05098] 初始化Debug相关参数
        (Variables|DebugVar|SetPrint%20INFO%20to%20Screen false)))
    (else
      (return))))

(fn DistanceCheck
  (params (Target :type Actor%20Object%20Reference))
  (return (<= (Transformation|GetDistanceTo Target) (Variables|CameraSystem|GetMax%20Detected%20Distance))))

(fn SlightCheck
  (params (Target :type BP%20SWGAS%20Character%20Object%20Reference))
  (bind _returnvalue (Collision|LineTraceForObjects (Transformation|GetActorLocation) (Transformation|GetActorLocation Target) (Utilities|Array|MakeArray "ObjectTypeQuery1") false (Utilities|Array|MakeArray Target) "None"))
  (return (not _returnvalue)))

(fn GetAllSWGASActor
  (bind _camera (Variables|Default|GetCamera))
  (Utilities|Map|Clear (Variables|CameraSystem|GetActors))
  (Utilities|Array|Clear (Variables|CameraSystem|GetCurrent%20Roatation))
  (bind _outactors (Actor|GetAllActorsOfClass "BP_SWGASCharacter_C"))
  (for _array_element _outactors
    (if (Math|Boolean|ANDBoolean (CameraSystem|DistanceCheck _array_element) (CameraSystem|SlightCheck _array_element) (!= _array_element self) (not (Variables|/Script/SwitchWeapon.SwitchWeaponCharacterBase|GetbIsShadow _array_element)))
      (Utilities|Map|Add (LocalVariables|GetLocal%20Actors) _array_element (Math|Float|Absolute(Float) (- (.yaw (Math|Rotator|FindLookatRotation (Transformation|GetWorldLocation _camera) (Transformation|GetActorLocation _array_element))) (.yaw (Math|Rotator|FindLookatRotation (Transformation|GetWorldLocation _camera) (Transformation|GetActorLocation))))))))
  (while (Utilities|Map|IsNotEmpty (LocalVariables|GetLocal%20Actors))
    (bind _values (Utilities|Map|Values (LocalVariables|GetLocal%20Actors)))
    (bind _keys (Utilities|Map|Keys (LocalVariables|GetLocal%20Actors)))
    (Utilities|Map|Add (Variables|CameraSystem|GetActors) (Utilities|Array|Get(acopy) _keys (.IndexOfMinValue (Math|Float|MinOfFloatArray _values))) (.MinValue (Math|Float|MinOfFloatArray _values)))
    (Utilities|Array|Add (Variables|CameraSystem|GetCurrent%20Roatation) (Math|Float|Absolute(Float) (.MinValue (Math|Float|MinOfFloatArray _values))))
    (Utilities|Map|Remove (LocalVariables|GetLocal%20Actors) (Utilities|Array|Get(acopy) _keys (.IndexOfMinValue (Math|Float|MinOfFloatArray _values))))
    (Development|PrintString (Utilities|String|ToString(Float) (Math|Float|Absolute(Float) (.MinValue (Math|Float|MinOfFloatArray _values))))))
  (return (Utilities|Map|IsNotEmpty (Variables|CameraSystem|GetActors))))

(fn SetCameraRotationMode
  (params (Use%20Controller%20Rotation%20Yaw :type Boolean) (Use%20Controller%20Desired%20Rotation :type Boolean) (Orient%20Rotation%20to%20Movement :type Boolean))
  (bind _self self)
  (bind _charactermovement (Variables|/Script/Engine.Character|GetCharacterMovement _self))
  (Variables|/Script/Engine.Pawn|SetbUseControllerRotationYaw _self Use%20Controller%20Rotation%20Yaw)
  (Variables|/Script/Engine.CharacterMovementComponent|SetbUseControllerDesiredRotation _charactermovement Use%20Controller%20Desired%20Rotation)
  (Variables|/Script/Engine.CharacterMovementComponent|SetbOrientRotationToMovement _charactermovement Orient%20Rotation%20to%20Movement))

(fn CameraTargetSwitch
  (LocalVariables|SetCopy%20of%20Current%20Target (Variables|CameraSystem|GetCurrentTarget))
  (if (Utilities|Map|IsNotEmpty (Variables|CameraSystem|GetActors))
    (bind _keys (Utilities|Map|Keys (Variables|CameraSystem|GetActors)))
    (if (== (Utilities|Array|FindItem _keys (Variables|CameraSystem|GetCurrentTarget)) (Utilities|Array|LastIndex _keys))
      ;[1 1 1] 重置锁定
      (bind _keys_2 (Utilities|Map|Keys (Variables|CameraSystem|GetActors)))
      (CallFunction|LockOff)
      (CallFunction|Lockon (Utilities|Array|Get(acopy) _keys_2))
      (else
        ;[1 1 1] 锁定下一个
        (bind _keys_3 (Utilities|Map|Keys (Variables|CameraSystem|GetActors)))
        (CallFunction|LockOff)
        (CallFunction|Lockon (Utilities|Array|Get(acopy) _keys_3 (+ (Utilities|Array|FindItem _keys_3 (LocalVariables|GetCopy%20of%20Current%20Target)) 1)))))))
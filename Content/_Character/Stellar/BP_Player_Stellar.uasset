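; BP_Player_Stellar is the Stellar player character, a thin child Blueprint that leaves input-action handling and construction to its parent.
; On BeginPlay it registers the blade mesh and a box collision with the attack trace component.
; A debug key sends the Event.Shadow gameplay event to itself.
; Unconnected leftover nodes for playing and stopping a sword clang sound never run.
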(event EventBeginPlay
  (|CallParentFunction)
  (Default|AddTraceMesh (Variables|Default|GetBPC_AttackTrace) (Variables|Default|GetSK_Blade) (Variables|Default|GetBox)))

(event Collision|EventActorBeginOverlap
  (params (OtherActor :type Actor%20Object%20Reference)))

(event EventTick
  (params (DeltaSeconds :type Float%20%28single-precision%29))
  (|CallParentFunction DeltaSeconds) ; This node is disabled and will not be called.\nDrag off pins to build functionality.
)

(event Input|KeyboardEvents|DebugKey3
  (params (Key :type Key%20Structure :default "None") (ActionValue :type Input%20Action%20Value%20Structure))
  (:Pressed
    (Ability|SendGameplayEventtoActor self "(TagName=\"Event.Shadow\")")))

(event Input|MouseEvents|LeftMouseButton
  (params (Key :type Key%20Structure :default "None")))

(fn ConstructionScript
  (|CallParentFunction))

(fn HandleInputAction
  (params (InputAction%20Tag :type Gameplay%20Tag%20Structure) (Tag%20Exists :type Boolean))
  (|CallParentFunction InputAction%20Tag Tag%20Exists))
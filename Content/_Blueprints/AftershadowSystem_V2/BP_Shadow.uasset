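; Afterimage of the owning player that replays an ability montage, then sends Event.Shadow.Done and destroys itself.
; It rebuilds a source mesh and its weapons with a dynamic shadow material and registers the weapon for attack tracing.
; Blank shadows freeze in the owner's montage pose until hit, then fade via timeline, take the attacker's appearance and replay its executed ability.
; The owner's lock-on event supplies the target for montage-time rotation.
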(event `Update Character Rotation`
  (params (`Delta Time` :type "Float (double-precision)"))
  ;[0.05098 0.05098 0.05098] ANS驱动，调整角色在montage中的朝向
  (bind _current_target (`self.Current Target`)
    (:`then`
      (bind _returnvalue (`self.K2_GetActorRotation` _current_target))
      (bind (_returnvalue_roll _returnvalue_pitch _returnvalue_yaw) (`KismetMathLibrary.BreakRotator` (`KismetMathLibrary.FindLookAtRotation` (`self.K2_GetActorLocation`) (`self.K2_GetActorLocation` _current_target))))
      (`self.K2_SetActorRotation` (`KismetMathLibrary.RInterpTo` _returnvalue (`KismetMathLibrary.MakeRotator` (.roll _returnvalue) (.pitch _returnvalue) _returnvalue_yaw) `Delta Time` 100.0)))
    (:`else`)))

(event `self.ReceiveBeginPlay`
  (bind _returnvalue (`SkeletalMeshComponent.GetAnimInstance` (`self.Mesh`)))
  (`|ExecutionSequence`
    (:`then_0`
      (`self.Init Shadow from Info`))
    (:`then_1`
      ;[0.05098 0.05098 0.05098] 实现和玩家蓝图通信，用于锁定/解锁目标
      (bind _asbp_swgascharacter (cast `/Game/_Character/BP_SWGASCharacter` (`self.GetOwner`)))
      (add `/Game/_Character/BP_SWGASCharacter.On Target Lock On` _asbp_swgascharacter (delegate `On Target Lock On_Event`)))
    (:`then_2`
      ;[0.05098 0.05098 0.05098] 空白残影初始化
      (if (`self.Is Blank`)
        (bind _asbp_swgascharacter_2 (cast `/Game/_Character/BP_SWGASCharacter` (`self.GetOwner`)))
        (bind _returnvalue_2 (`SkeletalMeshComponent.GetAnimInstance` (`Character.Mesh` _asbp_swgascharacter_2)))
        (bind _returnvalue_3 (`AnimInstance.GetCurrentActiveMontage` _returnvalue_2))
        (`self.PlayAnimMontage` _returnvalue_3)
        (`AnimInstance.Montage_SetPosition` _returnvalue _returnvalue_3 (`AnimInstance.Montage_GetPosition` _returnvalue_2 _returnvalue_3))
        (`AnimInstance.Montage_Pause` _returnvalue _returnvalue_3)
        (else
          ;[0.05098 0.05098 0.05098] 非空白残影直接释放动作
          (bind _asbp_swgascharacter_3 (cast `/Game/_Character/BP_SWGASCharacter` (`self.GetOwner`)))
          (bind _returnvalue_4 (`self.PlayAnimMontage` (`.AnimMontage` (`/Game/_Blueprints/AftershadowSystem_V2/CommonAbilityInfo.Get Info` (`/Game/_Character/BP_SWGASCharacter.Shadow Ability Info` _asbp_swgascharacter_3)))))
          (`KismetSystemLibrary.Delay` _returnvalue_4)
          (`AbilitySystemBlueprintLibrary.SendGameplayEventToActor` (`self.GetOwner`) (struct :`TagName` "Event.Shadow.Done"))
          (`self.K2_DestroyActor`))))))

(event `On Target Lock On_Event`
  (params (`Target Actor` :type "/Game/_Character/BP_SWGASCharacter Object Reference"))
  ;[0.05098 0.05098 0.05098] 实现和玩家蓝图通信，用于锁定/解锁目标
  (set `self.Current Target` `Target Actor`))

(event `Init Shadow from Info`
  (bind _bpc_attacktrace (`self.BPC_AttackTrace`))
  ;[0.05098 0.05098 0.05098] 初始化残影
  (`PrimitiveComponent.SetCollisionEnabled` (`self.CapsuleComponent`) "NoCollision")
  (for _array_element (`SceneComponent.GetChildrenComponents` (`self.Mesh`) false)
    (`ActorComponent.K2_DestroyComponent` _array_element))
  (`SkeletalMeshComponent.SetSkeletalMeshAsset` (`self.Mesh`) (`self.Src SK Mesh`))
  (for _array_element_2 (`SceneComponent.GetChildrenComponents` (`self.Src Mesh`) false)
    (bind (_weapon_box_ref _weapon_ref) (`self.Init Weapon` _array_element_2))
    (`PrimitiveComponent.SetCollisionEnabled` _weapon_box_ref "NoCollision")
    (`PrimitiveComponent.SetCollisionEnabled` _weapon_ref "NoCollision")
    (`SceneComponent.K2_AttachToComponent` _weapon_ref (`self.Mesh`) (`SceneComponent.GetAttachSocketName` _array_element_2) "KeepRelative" "KeepRelative" "KeepRelative" true))
  (`self.Init Shadow Material`)
  (`/Game/_Blueprints/CombatSystem/BPC_AttackTrace.Add Trace Mesh` _bpc_attacktrace _weapon_ref _weapon_box_ref)
  (`/Game/_Blueprints/CombatSystem/BPC_AttackTrace.Add Actor To Ignore` _bpc_attacktrace (`self.GetOwner`)))

(event `/Game/_Blueprints/CombatSystem/BPI_Attackable.On Hit`
  (params (Attacker :type "/Game/_Character/BP_SWGASCharacter Object Reference"))
  (bind _mesh (`Character.Mesh` Attacker))
  (if (`self.Is Blank`)
    (`/Engine/EditorBlueprintResources/StandardMacros.DoOnce` false
      (:`Completed`
        (bind (_direction _mask) (`Timeline|Timeline` :!via `ReverseFromEnd`)
          (:`Update`
            ;[0.05098 0.05098 0.05098] 空白残影特效
            (`MaterialInstanceDynamic.SetScalarParameterValue` (`self.Shadow Dynamic Material`) "Mask" _mask))
          (:`Finished`
            ;[0.05098 0.05098 0.05098] 空白残影攻击激活逻辑
            (if (`self.Is Blank`)
              (set `self.Is Blank` false)
              (set `self.Last Capsule Half Height` (`CapsuleComponent.GetScaledCapsuleHalfHeight` (`self.CapsuleComponent`)))
              (set `self.Src SK Mesh` (`SkeletalMeshComponent.GetSkeletalMeshAsset` _mesh))
              (set `self.Src Mesh` _mesh)
              (`SceneComponent.SetWorldScale3D` (`self.RootComponent`) (`SceneComponent.K2_GetComponentScale` (`Actor.RootComponent` Attacker)))
              (`self.Init Shadow from Info`)
              (`self.K2_SetActorLocation` (+ (* (`CapsuleComponent.GetScaledCapsuleHalfHeight` (`Character.CapsuleComponent` Attacker)) (`self.GetActorUpVector`)) (+ (`self.K2_GetActorLocation`) (* (`self.GetActorUpVector`) (* (`self.Last Capsule Half Height`) -1.0)))))
              (bind _returnvalue (`self.PlayAnimMontage` (`.AnimMontage_15_C03AA0A1457695A0229E5AA4E5574714` (break `/Game/_Blueprints/CombatSystem/Structure/S_SingleAbilityInfo` (`/Game/_Character/BP_SWGASCharacter.Excuted Ability Info` Attacker)))))
              (`KismetSystemLibrary.Delay` _returnvalue)
              (`AbilitySystemBlueprintLibrary.SendGameplayEventToActor` (`self.GetOwner`) (struct :`TagName` "Event.Shadow.Done"))
              (`self.K2_DestroyActor`))))))))

(fn `Init Shadow Material`
  (bind _mesh (`self.Mesh`))
  (bind _returnvalue (`KismetMaterialLibrary.CreateDynamicMaterialInstance` (`self.Shadow Material`) "Shadow Instance"))
  (set `self.Shadow Dynamic Material` _returnvalue)
  (`PrimitiveComponent.SetMaterial` _mesh 0 _returnvalue)
  (for _array_element (`SceneComponent.GetChildrenComponents` _mesh false)
    (bind `_as基元组件` (cast `PrimitiveComponent` _array_element))
    (`PrimitiveComponent.SetMaterial` `_as基元组件` 0 _returnvalue))
  (return))

(fn `Init Weapon`
  (params (Weapon :type "SceneComponent Object Reference"))
  (returns (`Weapon Box Ref` :type "BoxComponent Object Reference") (`Weapon Ref` :type "PrimitiveComponent Object Reference"))
  (bind _returnvalue (`SceneComponent.GetChildComponent` Weapon 0))
  (bind _relativescale3d (`SceneComponent.RelativeScale3D` Weapon))
  (bind `_as骨骼网格体组件` (cast `SkeletalMeshComponent` Weapon)
    (:`then`
      (bind _returnvalue_2 (`|AddComponentByClass` (`GameplayStatics.GetObjectClass` `_as骨骼网格体组件`) false (`KismetMathLibrary.MakeTransform` (0.0 0.0 0.0) (struct) _relativescale3d)))
      (`SkeletalMeshComponent.SetSkeletalMeshAsset` _returnvalue_2 (`SkeletalMeshComponent.SkeletalMeshAsset` `_as骨骼网格体组件`))
      (bind (__success _weapon_box_ref) (`self.Init Weapon Box` _returnvalue _returnvalue_2))
      (if __success
        (return _weapon_box_ref _returnvalue_2)))
    (:`CastFailed`
      (bind `_as静态网格体组件` (cast `StaticMeshComponent` Weapon))
      (bind _returnvalue_3 (`|AddComponentByClass` (`GameplayStatics.GetObjectClass` `_as静态网格体组件`) false (`KismetMathLibrary.MakeTransform` (0.0 0.0 0.0) (struct) _relativescale3d)))
      (`StaticMeshComponent.SetStaticMesh` _returnvalue_3 (`StaticMeshComponent.StaticMesh` `_as静态网格体组件`))
      (bind (__success_2 _weapon_box_ref_2) (`self.Init Weapon Box` _returnvalue _returnvalue_3))
      (if __success_2
        (return _weapon_box_ref_2 _returnvalue_3)))))

(fn `Init Weapon Box`
  (params (`Src Box` :type "Object Object Reference") (Parent :type "SceneComponent Object Reference"))
  (returns (`?Success` :type Boolean) (`Weapon Box Ref` :type "BoxComponent Object Reference"))
  (bind `_as盒体碰撞` (cast `BoxComponent` `Src Box`)
    (:`then`
      (bind _returnvalue (`|AddComponentByClass` (`GameplayStatics.GetObjectClass` `_as盒体碰撞`) false (`KismetMathLibrary.MakeTransform` (0.0 0.0 0.0) (struct) (`SceneComponent.RelativeScale3D` `_as盒体碰撞`))))
      (`BoxComponent.SetBoxExtent` _returnvalue (`BoxComponent.BoxExtent` `_as盒体碰撞`) true)
      (`SceneComponent.K2_AttachToComponent` _returnvalue Parent "None" "KeepRelative" "KeepRelative" "KeepRelative" true)
      (`SceneComponent.K2_SetRelativeTransform` _returnvalue (`SceneComponent.GetRelativeTransform` `_as盒体碰撞`) false false)
      (return true _returnvalue))
    (:`CastFailed`
      (return false null))))

(fn `UserConstructionScript`
  (`parent.UserConstructionScript`))
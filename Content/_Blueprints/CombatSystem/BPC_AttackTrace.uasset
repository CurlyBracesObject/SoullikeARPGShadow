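; Melee attack trace component for GAS characters and their shadows, detecting weapon hits during attacks.
; While tracing, a fast looping timer box-sweeps the weapon's collision box from previous to current position, hitting each actor once per attack.
; Hits send OnHitMessage, plus a damage gameplay event to GAS characters.
; Once per attack, montage-rate hit stop and directional camera shake follow HitForce and AttackFrom; non-players trigger these only on character hits.
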(event `self.ReceiveBeginPlay`
  (`|ExecutionSequence`
    (:`then_0`
      (bind `_as角色` (cast `Character` (`self.GetOwner`)))
      (bind _output_get (set `self.Owner` `_as角色`))
      ;[0.05098 0.05098 0.05098] 为项目单独准备的部分
      (bind _asbp_swgascharacter (cast `/Game/_Character/BP_SWGASCharacter` _output_get)
        (:`then`
          (bind _output_get_2 (set `self.GASCharacter` _asbp_swgascharacter))
          (set `self.BPC Switch Weapon ASC` (`/Game/_Character/BP_SWGASCharacter.BPC_SwitchWeaponASC` _asbp_swgascharacter))
          (cast `/Game/_Character/BP_Player_Test` _output_get_2
            (:`then`
              (set `self.IsPlayer` true))
            (:`CastFailed`
              (cast `/Game/AI/AI_Base/BP_EnmyBase` _output_get_2)
              (set `self.IsPlayer` false))))
        (:`CastFailed`
          (bind _asbp_shadow (cast `/Game/_Blueprints/AftershadowSystem_V2/BP_Shadow` _output_get))
          (bind _asbp_swgascharacter_2 (cast `/Game/_Character/BP_SWGASCharacter` (`Actor.GetOwner` _asbp_shadow)))
          (set `self.GASCharacter` _asbp_swgascharacter_2))))
    (:`then_1`
      (bind _returnvalue (`GameplayStatics.GetActorOfClass` "/Game/_Character/Stellar/BP_Player_Stellar.BP_Player_Stellar_C"))
      (set `self.Player` _returnvalue))))

(event `End Attack Trace`
  (bind _camera_shake_scale (`self.Camera Shake Scale`))
  (bind (_excuted_ability_info_ability _excuted_ability_info_animmontage _excuted_ability_info_triggerinputactiontag _excuted_ability_info_combotag _excuted_ability_info_dodgedirecitontag _excuted_ability_info_hitdirection _excuted_ability_info_hitforce _excuted_ability_info_damageinfo) (break `/Game/_Blueprints/CombatSystem/Structure/S_SingleAbilityInfo` (`/Game/_Character/BP_SWGASCharacter.Excuted Ability Info` (`self.GASCharacter`))))
  (bind (_damage _hitforce _attackfrom) (break `/Game/_Blueprints/CombatSystem/Structure/S_CommonDamageInfo` _excuted_ability_info_damageinfo))
  ;[0.05098 0.05098 0.05098] 关闭攻击检测
  (`KismetSystemLibrary.K2_ClearAndInvalidateTimerHandle` (stale `Start Attack Trace` _returnvalue))
  ;;[1 1 1] 清空上一轮攻击的命中结果
  (`KismetArrayLibrary.Array_Clear` (`self.Already Hit Actor`))
  (goto _label :!via `Reset`))

(event `Start Attack Trace`
  ;[0.05098 0.05098 0.05098] 开启攻击检测
  (`self.Update Box Collision Location`)
  (bind _returnvalue (`KismetSystemLibrary.K2_SetTimerDelegate` (delegate `On Attack Trace`) 0.01 true)))

(event `On Attack Trace`
  (bind _owner (`self.Owner`))
  (bind _gascharacter (`self.GASCharacter`))
  (bind (_weapon_index _weapon_weaponmesh _weapon_boxcollision) (break `/Game/_Blueprints/CombatSystem/Structure/S_SingleWeapon` (`self.Weapon`)))
  (bind _camera_shake_scale (`self.Camera Shake Scale`))
  (bind (_excuted_ability_info_ability _excuted_ability_info_animmontage _excuted_ability_info_triggerinputactiontag _excuted_ability_info_combotag _excuted_ability_info_dodgedirecitontag _excuted_ability_info_hitdirection _excuted_ability_info_hitforce _excuted_ability_info_damageinfo) (break `/Game/_Blueprints/CombatSystem/Structure/S_SingleAbilityInfo` (`/Game/_Character/BP_SWGASCharacter.Excuted Ability Info` (`self.GASCharacter`))))
  (bind (_excuted_ability_info_ability_2 _excuted_ability_info_animmontage_2 _excuted_ability_info_triggerinputactiontag_2 _excuted_ability_info_combotag_2 _excuted_ability_info_dodgedirecitontag_2 _excuted_ability_info_hitdirection_2 _excuted_ability_info_hitforce_2 _excuted_ability_info_damageinfo_2) (break `/Game/_Blueprints/CombatSystem/Structure/S_SingleAbilityInfo` (`/Game/_Character/BP_SWGASCharacter.Excuted Ability Info` (`self.GASCharacter`))))
  (bind (_excuted_ability_info_ability_3 _excuted_ability_info_animmontage_3) (break `/Game/_Blueprints/CombatSystem/Structure/S_SingleAbilityInfo` (`/Game/_Character/BP_SWGASCharacter.Excuted Ability Info` _gascharacter)))
  (bind (_damage _hitforce _attackfrom) (break `/Game/_Blueprints/CombatSystem/Structure/S_CommonDamageInfo` _excuted_ability_info_damageinfo_2))
  (bind (_damage_2 _hitforce_2) (break `/Game/_Blueprints/CombatSystem/Structure/S_CommonDamageInfo` _excuted_ability_info_damageinfo))
  (if (`self.Should Check?`)
    (bind _last_location (`self.Update Box Collision Location`))
    (bind (_outhits _returnvalue) (`KismetSystemLibrary.BoxTraceMultiForObjects` _last_location (`self.Box Location`) (`BoxComponent.BoxExtent` _weapon_boxcollision) (`SceneComponent.K2_GetComponentRotation` _weapon_boxcollision) (`|MakeArray` "ObjectTypeQuery1" "ObjectTypeQuery2" "ObjectTypeQuery3" :!type "EObjectTypeQuery Enum") false (`self.Actors to Ignore`) (`self.Draw Debug Type`) true (struct :`R` 1.0 :`A` 1.0) (struct :`G` 1.0 :`A` 1.0) (`self.Draw Time`)))
    (if _returnvalue
      (for _array_element _outhits
        (bind _output_get (set `self.Last Hit` _array_element))
        (bind (_bblockinghit _binitialoverlap _time _distance _location _impactpoint _normal _impactnormal _physmat _hitactor) (`GameplayStatics.BreakHitResult` _output_get))
        ;[0.05098 0.05098 0.05098] 如果对象已经被击中过，在结束攻击之前不会再次被击中
        (if (not (`KismetArrayLibrary.Array_Contains` (`self.Already Hit Actor`) _hitactor))
          (`|ExecutionSequence`
            (:`then_0`
              ;[0.05098 0.05098 0.05098] 通知除SW GAS Character之外的Actor接受伤害
              (message `/Game/_Blueprints/CombatSystem/BPI_Attackable.On Hit` _hitactor (`self.GASCharacter`)))
            (:`then_1`
              (bind _output_get_2 (set `self.Hit Actor` _hitactor))
              (`KismetArrayLibrary.Array_Add` (`self.Already Hit Actor`) _output_get_2))
            (:`then_2`
              (bind _asbp_swgascharacter (cast `/Game/_Character/BP_SWGASCharacter` _hitactor))
              (`|ExecutionSequence`
                (:`then_0`
                  (bind _returnvalue_2 (`|GenericCreateObject` _owner "/Game/_Blueprints/AftershadowSystem_V2/CommonAbilityInfo.CommonAbilityInfo_C"))
                  (`/Game/_Blueprints/AftershadowSystem_V2/CommonAbilityInfo.Set Info` _returnvalue_2 _gascharacter _excuted_ability_info_ability_3 _excuted_ability_info_animmontage_3 (`CapsuleComponent.GetScaledCapsuleHalfHeight` (`Character.CapsuleComponent` _gascharacter))))
                (:`then_1`
                  (bind _returnvalue_3 (`|GenericCreateObject` _owner "/Game/_Blueprints/CombatSystem/CommonDamageInfo.CommonDamageInfo_C"))
                  (`/Game/_Blueprints/CombatSystem/CommonDamageInfo.Set Info` _returnvalue_3 _damage_2 _hitforce_2))
                (:`then_2`
                  (`AbilitySystemBlueprintLibrary.SendGameplayEventToActor` _asbp_swgascharacter (struct :`TagName` "Event.HandleDamage") (make `GameplayEventData` (struct :`TagName` "Event.MeleeAttack") (`self.Owner`) _asbp_swgascharacter _returnvalue_2 _returnvalue_3 (struct) (struct) (`GameplayTagAssetInterface.GetOwnedGameplayTags` (`AbilitySystemBlueprintLibrary.GetAbilitySystemComponent` _asbp_swgascharacter)) 0.0 (`AbilitySystemBlueprintLibrary.AbilityTargetDataFromHitResult` (`self.Last Hit`)))))
                (:`then_3`
                  ;[1 1 1] 怪物只有击中目标才能发生震屏
                  (if (not (`self.IsPlayer`))
                    (`/Engine/EditorBlueprintResources/StandardMacros.DoOnce` false :!label _label
                      (:`Completed`
                        (`|ExecutionSequence`
                          (:`then_0`
                            (switch `/Game/_Blueprints/CombatSystem/Enum/E_HitDegree` _hitforce
                              (:`NewEnumerator0`
                                (`self.卡肉` 0.0001 0.03)
                                (set `self.Camera Shake Scale` 1.0))
                              (:`NewEnumerator1`
                                (`self.卡肉` 0.0001 0.12)
                                (set `self.Camera Shake Scale` 2.0))))
                          (:`then_1`
                            (bind `_as玩家控制器` (cast `PlayerController` (`Actor.GetOwner` (`self.Player`))))
                            (switch `/Game/_Blueprints/CombatSystem/Enum/E_AttackDirection` _attackfrom
                              (:`NewEnumerator0`
                                (bind _playercameramanager (`PlayerController.PlayerCameraManager` `_as玩家控制器`))
                                (`PlayerCameraManager.StartCameraShake` :`self` _playercameramanager :`ShakeClass` "/Game/_Blueprints/CameraSystem/BP_CameraShake_Horizontal.BP_CameraShake_Horizontal_C" :`Scale` _camera_shake_scale))
                              (:`NewEnumerator1`
                                (`PlayerCameraManager.StartCameraShake` :`self` _playercameramanager :`ShakeClass` "/Game/_Blueprints/CameraSystem/BP_CameraShake_Vertical.BP_CameraShake_Vertical_C" :`Scale` _camera_shake_scale))
                              (:`NewEnumerator2`
                                (`PlayerCameraManager.StartCameraShake` :`self` _playercameramanager :`ShakeClass` "/Game/_Blueprints/CameraSystem/BP_CameraShake_FrontBack.BP_CameraShake_FrontBack_C" :`Scale` _camera_shake_scale)))))))))))
            (:`then_3`
              (if (`self.IsPlayer`)
                (goto _label)))))))))

(event `卡肉`
  (params (NewPlayRate :type "Float (single-precision)") (Duration :type "Float (single-precision)"))
  (`AnimInstance.Montage_SetPlayRate` (`SkeletalMeshComponent.GetAnimInstance` (`Character.Mesh` (`self.Owner`))) null NewPlayRate)
  (`KismetSystemLibrary.Delay` Duration)
  (`AnimInstance.Montage_SetPlayRate` (`SkeletalMeshComponent.GetAnimInstance` (`Character.Mesh` (`self.Owner`))) null 1.2))

(event `顿帧`
  (bind _returnvalue (`SkeletalMeshComponent.GetAnimInstance` (`Character.Mesh` (`self.Owner`))))
  ;[0.05098 0.05098 0.05098] 目前看下来效果不是特别好
  (set `self.Duration` (`KismetMathLibrary.RandomFloatInRange` 0.02 0.04))
  (`AnimInstance.Montage_Pause` _returnvalue null)
  (`KismetSystemLibrary.Delay` (`self.Duration`))
  (`AnimInstance.Montage_Resume` _returnvalue null)
  (`AnimInstance.Montage_SetPlayRate` _returnvalue null 1.2))

(fn `Add Actor To Ignore`
  (params (`Add Actor` :type "Actor Object Reference (by ref)"))
  (`KismetArrayLibrary.Array_AddUnique` (`self.Actors to Ignore`) `Add Actor`))

(fn `Add Trace Mesh`
  (params (`Trace Mesh` :type "PrimitiveComponent Object Reference") (`Box Collision` :type "BoxComponent Object Reference"))
  ;[1 1 1] 之后考虑升级成可以加入多个武器的
  (set `self.Weapon` (make `/Game/_Blueprints/CombatSystem/Structure/S_SingleWeapon` 0 `Trace Mesh` `Box Collision`)))

(fn `Get Actor To lgnore`
  (returns (`Actors to Ignore` :type "Array of Actor Object Reference"))
  (return (`self.Actors to Ignore`)))

(fn `Get Already Hit Actor`
  (returns (`Already Hit Actor` :type "Array of Actor Object Reference"))
  (return (`self.Already Hit Actor`)))

(fn `Get Last Hit`
  (returns (`Last Hit` :type "HitResult Structure"))
  (return (`self.Last Hit`)))

(fn `Get Trace Mesh`
  (returns (Weapon :type "/Game/_Blueprints/CombatSystem/Structure/S_SingleWeapon Structure"))
  (return (`self.Weapon`)))

(fn `Get Weapon Box`)

(fn `Remove Actor To lgnore`
  (params (`Remove Actor` :type "Actor Object Reference (by ref)"))
  (returns (`Is Success?` :type Boolean))
  (bind _returnvalue (`KismetArrayLibrary.Array_RemoveItem` (`self.Actors to Ignore`) `Remove Actor`))
  (return _returnvalue))

(fn `Update Box Collision Location`
  (returns (`Last Location` :type "Vector Structure"))
  (locals (`Pre Box Location` :type "Vector Structure"))
  (bind (_weapon_index _weapon_weaponmesh _weapon_boxcollision) (break `/Game/_Blueprints/CombatSystem/Structure/S_SingleWeapon` (`self.Weapon`)))
  (`|ExecutionSequence`
    (:`then_0`
      ;[1 1 1] 记录之前的位置
      (set `local.Pre Box Location` (`self.Box Location`)))
    (:`then_1`
      ;[1 1 1] 更新一次当前的位置
      (set `self.Box Location` (`SceneComponent.K2_GetComponentLocation` _weapon_boxcollision)))
    (:`then_2`
      (return (`local.Pre Box Location`)))))
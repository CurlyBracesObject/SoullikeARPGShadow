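; Base enemy AI Blueprint that handles player detection, health display and death.
; Perception updates the blackboard "Player" key, current target and widget visibility, skipping detection when either side is a shadow.
; Tick feeds GAS attributes to the health bar and, at zero, triggers death: animation, colored Niagara effect, dissolve material swap and delayed destruction.
; A timeline smoothly blends walk speed and can be interrupted.
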(event `self.ReceiveBeginPlay`
  (`parent.ReceiveBeginPlay`))

(event `Reset Speed Smoothly AI`
  (params (`New Walk Speed` :type "Float (double-precision)"))
  ;[0.05098 0.05098 0.05098] 缓慢重设奔跑回复的速度AI
  (set `self.Last Max Walk Speed` (`CharacterMovementComponent.MaxWalkSpeed` (`self.CharacterMovement`)))
  (bind (_direction _newtrack_0) (`Timeline|Timeline_2` :!via `PlayFromStart` :!label _label)
    (:`Update`
      (bind _output_get (set `CharacterMovementComponent.MaxWalkSpeed` (`KismetMathLibrary.Lerp` (`self.Last Max Walk Speed`) `New Walk Speed` _newtrack_0) (`self.CharacterMovement`)))
      (`KismetSystemLibrary.PrintString` (`KismetStringLibrary.Conv_DoubleToString` _output_get) true true (struct :`G` 0.66 :`B` 1.0 :`A` 1.0) 2.0 "AI Speed"))))

(event `Reactivate During Changing AI`
  ;[0.05098 0.05098 0.05098] 缓慢重设奔跑回复的速度AI
  (goto _label :!via `Stop`))

(event `self.AIPerception.OnTargetPerceptionUpdated`
  (params (Actor :type "Actor Object Reference") (Stimulus :type "AIStimulus Structure"))
  (bind _widget (`self.Widget`))
  (if (not (`self.bIsShadow`))
    (bind _asbp_player_test (cast `/Game/_Character/BP_Player_Test` Actor))
    (if (not (`SwitchWeaponCharacterBase.bIsShadow` _asbp_player_test))
      (if (`.bSuccessfullySensed` (break `AIStimulus` Stimulus))
        (`BlackboardComponent.SetValueAsObject` (`AIBlueprintHelperLibrary.GetBlackboard` null) "Player" _asbp_player_test)
        (set `self.CurrentTarget` _asbp_player_test)
        (`SceneComponent.ToggleVisibility` _widget true)
        (else
          (`BlackboardComponent.SetValueAsObject` (`AIBlueprintHelperLibrary.GetBlackboard` null) "Player" null)
          (set `self.CurrentTarget` null)
          (`SceneComponent.ToggleVisibility` _widget false))))))

(event `self.ReceiveTick`
  (params (DeltaSeconds :type "Float (single-precision)"))
  (bind _returnvalue (/ (`.ReturnValue` (`AbilitySystemComponent.GetGameplayAttributeValue` (`self.BPC_SwitchWeaponASC`) (struct :`AttributeName` "Health" :`Attribute` "/Script/SwitchWeapon.SWAttributeSet:Health" :`AttributeOwner` "/Script/CoreUObject.Class'/Script/SwitchWeapon.SWAttributeSet'"))) (`.ReturnValue` (`AbilitySystemComponent.GetGameplayAttributeValue` (`self.BPC_SwitchWeaponASC`) (struct :`AttributeName` "MaxHealth" :`Attribute` "/Script/SwitchWeapon.SWAttributeSet:MaxHealth" :`AttributeOwner` "/Script/CoreUObject.Class'/Script/SwitchWeapon.SWAttributeSet'")))))
  (if (`self.死亡`)
    (`/Engine/EditorBlueprintResources/StandardMacros.DoOnce` false
      (:`Completed`
        (`self.死亡特效`)))
    (else
      (bind _asblood (cast `/Game/AI/AI_Base/Blood` (`WidgetComponent.GetWidget` (`self.Widget`))))
      (`/Game/AI/AI_Base/Blood.Set Percent` _asblood _returnvalue)
      (if (<= _returnvalue 0.0)
        (set `self.死亡` true)))))

(event `死亡特效`
  (bind _mesh (`self.Mesh`))
  (`CharacterMovementComponent.DisableMovement` (`self.CharacterMovement`))
  (`SkeletalMeshComponent.PlayAnimation` (`self.Mesh`) "/Game/Sword_Animations/Animations/Sequence/08_Hit/05_Hit_Large/Hit_Large_Death_Seq.Hit_Large_Death_Seq" false)
  (bind _returnvalue (`NiagaraFunctionLibrary.SpawnSystemAttached` (`self.System Template`) _mesh "None" (0.0 0.0 0.0) (struct) "KeepRelativeOffset"))
  (`NiagaraComponent.SetVariableVec3` _returnvalue "Color" (`KismetMathLibrary.Conv_LinearColorToVector` (`self.Color`)))
  (for (_ _array_index) (`MeshComponent.GetMaterials` _mesh)
    (`PrimitiveComponent.SetMaterial` (`self.Mesh`) _array_index (`self.DissolveMat`))
    (`KismetSystemLibrary.Delay` 2.0)
    (`self.K2_DestroyActor`)))

(fn `Dissole Mat Param`
  (params (Mesh :type "MeshComponent Object Reference") (AmountParameterValue :type "Float (double-precision)")))

(fn `UserConstructionScript`
  (`parent.UserConstructionScript`))